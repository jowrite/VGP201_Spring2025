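; BP_CharController routes player input to the left and right flippers in the level.
; On BeginPlay it finds all BP_Flipper actors and stores one reference per side based on each one's IsLeft flag.
; The FlipperLeft and FlipperRight input actions call OnPressed and OnRelease on the matching flipper, printing a debug string on each press.
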(event `self.ReceiveBeginPlay`
  (bind _outactors (`GameplayStatics.GetAllActorsOfClass` "/Game/Blueprints/BP_Flipper.BP_Flipper_C"))
  (for _array_element _outactors
    (if (`/Game/Blueprints/BP_Flipper.IsLeft` _array_element)
      (set `self.LeftFlipperReference` _array_element)
      (else
        (set `self.RightFlipperReference` _array_element)))))

(event `InputAction|FlipperRight`
  (params (Key :type "Key Structure"))
  (bind _rightflipperreference (`self.RightFlipperReference`))
  (:`Pressed`
    (`KismetSystemLibrary.PrintString` "Pressing Right")
    (`/Game/Blueprints/BP_Flipper.OnPressed` _rightflipperreference))
  (:`Released`
    (`/Game/Blueprints/BP_Flipper.OnRelease` _rightflipperreference)))

(event `InputAction|FlipperLeft`
  (params (Key :type "Key Structure"))
  (bind _leftflipperreference (`self.LeftFlipperReference`))
  (:`Pressed`
    (`KismetSystemLibrary.PrintString` "Pressing Left")
    (`/Game/Blueprints/BP_Flipper.OnPressed` _leftflipperreference))
  (:`Released`
    (`/Game/Blueprints/BP_Flipper.OnRelease` _leftflipperreference)))

(fn `UserConstructionScript`)